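; Player actor that moves in the world XZ plane from horizontal and vertical input, aims at the mouse cursor and spawns a BP_TestPoint on left click.
; Tick teleports it without sweep, then turns MeshParent toward the cursor trace hit flattened to the actor's Y, ignoring hits within a small dead zone.
; GetAngle and IsMouseUpPosition switch the rotation's Z reference from up to right vector when aim nears vertical.
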(event EventBeginPlay
  (Variables|/Script/Engine.PlayerController|SetbShowMouseCursor (Game|GetPlayerController 0) true))

(event Collision|EventActorBeginOverlap
  (params (OtherActor :type Actor%20Object%20Reference)))

(event EventTick
  (params (DeltaSeconds :type Float%20%28single-precision%29))
  (bind _returnvalue (Game|GetPlayerController 0))
  (bind _returnvalue_2 (Transformation|GetActorLocation))
  (bind _returnvalue_3 (Transformation|GetActorLocation))
  (bind _hitresult (Game|Player|GetHitResultUnderCursorbyChannel _returnvalue "TraceTypeQuery1" true))
  (bind _impactpoint (Collision|BreakHitResult _hitresult))
  (bind _returnvalue_4 (Math|Vector|MakeVector (.x _impactpoint) (.y _returnvalue_2) (.z _impactpoint)))
  (bind _returnvalue_5 (- _returnvalue_4 _returnvalue_3))
  (Utilities|FlowControl|Sequence
    (:then_0
      (CallFunction|Translate (Math|Vector|MakeVector (Input|AxisValues|GetHorizontal) 0.0 (Input|AxisValues|GetVertical)) (Variables|Default|Getspeed) DeltaSeconds))
    (:then_1
      (if (> (Math|Vector|VectorLength _returnvalue_5) 1e+02)
        (if (CallFunction|IsMouseUpPosition (CallFunction|GetAngle (Transformation|GetActorUpVector) _returnvalue_5))
          (bind _output_get (Variables|Default|SetnewRotation (Math|Rotator|MakeRotfromXZ _returnvalue_5 (Transformation|GetActorRightVector))))
          (Transformation|SetWorldRotation (Variables|Default|GetMeshParent) _output_get false false)
          (else
            (bind _output_get_2 (Variables|Default|SetnewRotation (Math|Rotator|MakeRotfromXZ _returnvalue_5 (Transformation|GetActorUpVector))))
            (Transformation|SetWorldRotation (Variables|Default|GetMeshParent) _output_get_2 false false)))))))

(event Input|ActionEvents|InputActionLeftMouse
  (params (Key :type Key%20Structure :default "None"))
  (:Pressed
    (Game|SpawnActorfromClass "/Game/TopDown/Blueprints/BP_TestPoint.BP_TestPoint_C" (Transformation|GetWorldTransform (Variables|Default|GetMeshParent)) "AlwaysSpawn" 0 0)))

(fn ConstructionScript)

(fn Translate
  (params (Direction :type Vector) (Speed :type Float%20%28double-precision%29) (DeltaTime :type Float%20%28double-precision%29))
  (Transformation|SetActorLocation (+ (Transformation|GetActorLocation) (* Direction Speed DeltaTime)) false true))

(fn GetAngle
  (params (A :type Vector) (B :type Vector))
  (bind _returnvalue (Math|Vector|Normalize B))
  (bind _returnvalue_2 (Math|Vector|Normalize A))
  (Utilities|FlowControl|Sequence
    (:then_0
      (LocalVariables|SetdegreeAngle (Math|Trig|RadiansToDegrees (Math|Trig|Acos(Degrees) (Math|Vector|DotProduct _returnvalue_2 _returnvalue))))
      (if (< (.z (Math|Vector|CrossProduct _returnvalue_2 _returnvalue)) 0.0)
        (LocalVariables|SetdegreeAngle (* (LocalVariables|GetdegreeAngle) -1.0))))
    (:then_1
      (return (LocalVariables|GetdegreeAngle)))))

(fn IsMouseUpPosition
  (params (angle :type Float%20%28double-precision%29))
  (return (Math|Boolean|ORBoolean (> angle 315.0) (< angle 45.0) (and (> angle 135.0) (< angle 225.0)))))